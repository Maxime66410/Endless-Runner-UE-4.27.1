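; BP_Obstacle19 is a minivan obstacle that kills the player's ThirdPersonCharacter on collision.
; Hit events on the BasVehicle and VitreVehicle components each cast the other actor to ThirdPersonCharacter and, if it is not already dead, set IsDead.
; Both paths share one 2D crash sound, which the IsDead check keeps from replaying on further hits.
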(event `self.BasVehicle.OnComponentHit`
  (params (HitComponent :type "PrimitiveComponent Object Reference") (OtherActor :type "Actor Object Reference") (OtherComp :type "PrimitiveComponent Object Reference") (NormalImpulse :type "Vector Structure") (Hit :type "HitResult Structure (by ref)"))
  (bind _asthird_person_character (cast `/Game/ThirdPersonBP/Blueprints/ThirdPersonCharacter` OtherActor))
  (if (not (`/Game/ThirdPersonBP/Blueprints/ThirdPersonCharacter.IsDead?` _asthird_person_character))
    (set `/Game/ThirdPersonBP/Blueprints/ThirdPersonCharacter.IsDead?` true _asthird_person_character)
    (`GameplayStatics.PlaySound2D` "/Game/Assets/Audio/Player/CrashCars.CrashCars" 1.0 1.0 0.0 null null :!label _label)))

(event `self.VitreVehicle.OnComponentHit`
  (params (HitComponent :type "PrimitiveComponent Object Reference") (OtherActor :type "Actor Object Reference") (OtherComp :type "PrimitiveComponent Object Reference") (NormalImpulse :type "Vector Structure") (Hit :type "HitResult Structure (by ref)"))
  (bind _asthird_person_character (cast `/Game/ThirdPersonBP/Blueprints/ThirdPersonCharacter` OtherActor))
  (if (not (`/Game/ThirdPersonBP/Blueprints/ThirdPersonCharacter.IsDead?` _asthird_person_character))
    (set `/Game/ThirdPersonBP/Blueprints/ThirdPersonCharacter.IsDead?` true _asthird_person_character)
    (goto _label)))

(fn `UserConstructionScript`)