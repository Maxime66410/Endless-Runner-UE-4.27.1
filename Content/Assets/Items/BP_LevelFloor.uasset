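; BP_LevelFloor is a road segment that carries a random obstacle or coin and keeps the level extending as the player advances.
; Its Construction Script gathers right, left and middle spawn transforms, builds the class list, then adds one random entry as a Child Actor Component at a random point.
; When ThirdPersonCharacter overlaps EndTrigger, it calls AddRoad on the BP_Generation actor cached at BeginPlay and destroys itself.
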(event `self.ReceiveBeginPlay`
  ;[1 1 1] Get BP_Generation
  (bind _returnvalue (`GameplayStatics.GetActorOfClass` "/Game/Assets/Items/BP_Generation.BP_Generation_C"))
  (set `self.GenerationCast` _returnvalue))

(event `self.End Trigger.OnComponentBeginOverlap`
  (params (OverlappedComponent :type "PrimitiveComponent Object Reference") (OtherActor :type "Actor Object Reference") (OtherComp :type "PrimitiveComponent Object Reference") (OtherBodyIndex :type Integer) (bFromSweep :type Boolean) (SweepResult :type "HitResult Structure (by ref)"))
  ;[1 1 1] If player hit, Add road + Destroy this actor
  (cast `/Game/ThirdPersonBP/Blueprints/ThirdPersonCharacter` OtherActor)
  (`/Game/Assets/Items/BP_Generation.AddRoad` (`self.GenerationCast`))
  (`self.K2_DestroyActor`))

(fn `SetObstacles`
  (set `self.Obstacles` (`|MakeArray` "/Game/Assets/Obstacle/Compact/BP_Obstacle01.BP_Obstacle01_C" "/Game/Assets/Obstacle/Compact/BP_Obstacle02.BP_Obstacle02_C" "/Game/Assets/Obstacle/Compact/BP_Obstacle03.BP_Obstacle03_C" "/Game/Assets/Obstacle/Compact/BP_Obstacle04.BP_Obstacle04_C" "/Game/Assets/Obstacle/Compact/BP_Obstacle05.BP_Obstacle05_C" "/Game/Assets/Obstacle/Coupe/BP_Obstacle06.BP_Obstacle06_C" "/Game/Assets/Obstacle/Coupe/BP_Obstacle07.BP_Obstacle07_C" "/Game/Assets/Obstacle/Coupe/BP_Obstacle08.BP_Obstacle08_C" "/Game/Assets/Obstacle/Coupe/BP_Obstacle08.BP_Obstacle08_C" "/Game/Assets/Obstacle/Coupe/BP_Obstacle09.BP_Obstacle09_C" "/Game/Assets/Obstacle/Coupe/BP_Obstacle10.BP_Obstacle10_C" "/Game/Assets/Obstacle/Hatchback/BP_Obstacle11.BP_Obstacle11_C" "/Game/Assets/Obstacle/Hatchback/BP_Obstacle12.BP_Obstacle12_C" "/Game/Assets/Obstacle/Hatchback/BP_Obstacle13.BP_Obstacle13_C" "/Game/Assets/Obstacle/Hatchback/BP_Obstacle14.BP_Obstacle14_C" "/Game/Assets/Obstacle/Hatchback/BP_Obstacle15.BP_Obstacle15_C" "/Game/Assets/Obstacle/Minivan/BP_Obstacle16.BP_Obstacle16_C" "/Game/Assets/Obstacle/Minivan/BP_Obstacle17.BP_Obstacle17_C" "/Game/Assets/Obstacle/Minivan/BP_Obstacle18.BP_Obstacle18_C" "/Game/Assets/Obstacle/Minivan/BP_Obstacle19.BP_Obstacle19_C" "/Game/Assets/Obstacle/Minivan/BP_Obstacle20.BP_Obstacle20_C" "/Game/Assets/Obstacle/Offroad/BP_Obstacle21.BP_Obstacle21_C" "/Game/Assets/Obstacle/Offroad/BP_Obstacle22.BP_Obstacle22_C" "/Game/Assets/Obstacle/Offroad/BP_Obstacle23.BP_Obstacle23_C" "/Game/Assets/Obstacle/Offroad/BP_Obstacle24.BP_Obstacle24_C" "/Game/Assets/Obstacle/Offroad/BP_Obstacle25.BP_Obstacle25_C" "/Game/Assets/Items/BP_Coin.BP_Coin_C" "/Game/Assets/Items/BP_CoinMedium.BP_CoinMedium_C" "/Game/Assets/Items/BP_CoinBig.BP_CoinBig_C" "/Game/Assets/Items/BP_CoinLarge.BP_CoinLarge_C" "/Game/Assets/Obstacle/Pickup/BP_Obstacle26.BP_Obstacle26_C" "/Game/Assets/Obstacle/Pickup/BP_Obstacle27.BP_Obstacle27_C" "/Game/Assets/Obstacle/Pickup/BP_Obstacle28.BP_Obstacle28_C" "/Game/Assets/Obstacle/Pickup/BP_Obstacle29.BP_Obstacle29_C" "/Game/Assets/Obstacle/Pickup/BP_Obstacle30.BP_Obstacle30_C" "/Game/Assets/Obstacle/Sedan/BP_Obstacle31.BP_Obstacle31_C" "/Game/Assets/Obstacle/Sedan/BP_Obstacle32.BP_Obstacle32_C" "/Game/Assets/Obstacle/Sedan/BP_Obstacle33.BP_Obstacle33_C" "/Game/Assets/Obstacle/Sedan/BP_Obstacle34.BP_Obstacle34_C" "/Game/Assets/Obstacle/Sedan/BP_Obstacle35.BP_Obstacle35_C" "/Game/Assets/Obstacle/Sport/BP_Obstacle36.BP_Obstacle36_C" "/Game/Assets/Obstacle/Sport/BP_Obstacle37.BP_Obstacle37_C" "/Game/Assets/Obstacle/Sport/BP_Obstacle38.BP_Obstacle38_C" "/Game/Assets/Obstacle/Sport/BP_Obstacle39.BP_Obstacle39_C" "/Game/Assets/Obstacle/Sport/BP_Obstacle40.BP_Obstacle40_C" "/Game/Assets/Obstacle/SUV/BP_Obstacle41.BP_Obstacle41_C" "/Game/Assets/Obstacle/SUV/BP_Obstacle42.BP_Obstacle42_C" "/Game/Assets/Obstacle/SUV/BP_Obstacle43.BP_Obstacle43_C" "/Game/Assets/Obstacle/SUV/BP_Obstacle44.BP_Obstacle44_C" "/Game/Assets/Obstacle/SUV/BP_Obstacle45.BP_Obstacle45_C" "/Game/Assets/Obstacle/Wagon/BP_Obstacle46.BP_Obstacle46_C" "/Game/Assets/Obstacle/Wagon/BP_Obstacle47.BP_Obstacle47_C" "/Game/Assets/Obstacle/Wagon/BP_Obstacle48.BP_Obstacle48_C" "/Game/Assets/Obstacle/Wagon/BP_Obstacle49.BP_Obstacle49_C" "/Game/Assets/Obstacle/Wagon/BP_Obstacle50.BP_Obstacle50_C" "/Game/Assets/Obstacle/Truck/BP_Obstacle51.BP_Obstacle51_C" "/Game/Assets/Obstacle/Truck/BP_Obstacle52.BP_Obstacle52_C" "/Game/Assets/Obstacle/Truck/BP_Obstacle53.BP_Obstacle53_C" "/Game/Assets/Obstacle/Truck/BP_Obstacle54.BP_Obstacle54_C" "/Game/Assets/Obstacle/Truck/BP_Obstacle55.BP_Obstacle55_C" "/Game/Assets/Obstacle/Bus/BP_Obstacle56.BP_Obstacle56_C" "/Game/Assets/Obstacle/Bus/BP_Obstacle57.BP_Obstacle57_C" "/Game/Assets/Obstacle/Bus/BP_Obstacle58.BP_Obstacle58_C" "/Game/Assets/Obstacle/Bus/BP_Obstacle59.BP_Obstacle59_C" "/Game/Assets/Obstacle/Bus/BP_Obstacle60.BP_Obstacle60_C" "/Game/Assets/Obstacle/Barriere/BP_Obstacle61.BP_Obstacle61_C" "/Game/Assets/Obstacle/Barriere/BP_Obstacle62.BP_Obstacle62_C" "/Game/Assets/Obstacle/Barriere/BP_Obstacle63.BP_Obstacle63_C" "/Game/Assets/Obstacle/Barriere/BP_Obstacle64.BP_Obstacle64_C" null :!type "Actor Class Reference")))

(fn `SetSpawnPoints`
  (set `self.SpawnPoints` (`|MakeArray` (`SceneComponent.GetRelativeTransform` (`self.SpawnR`)) (`SceneComponent.GetRelativeTransform` (`self.SpawnL`)) (`SceneComponent.GetRelativeTransform` (`self.SpawnM`)))))

(fn `SpawnObstacles`
  (bind _spawnpoints (`self.SpawnPoints`))
  (bind _obstacles (`self.Obstacles`))
  (bind _returnvalue (`AddComponent|NODE_AddChildActorComponent-0` :`RelativeTransform` (`|GetArrayItem` _spawnpoints (`KismetMathLibrary.RandomIntegerInRange` 0 (`KismetArrayLibrary.Array_LastIndex` _spawnpoints)))))
  (`ChildActorComponent.SetChildActorClass` _returnvalue (`|GetArrayItem` _obstacles (`KismetMathLibrary.RandomIntegerInRange` 0 (`KismetArrayLibrary.Array_LastIndex` _obstacles)))))

(fn `UserConstructionScript`
  (`self.SetSpawnPoints`) ; Update Spawn Points
  (`self.SetObstacles`) ; Get list of Obstacles
  (`self.SpawnObstacles`) ; Spawn Random obstacles in the list
)