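; BP_Generation builds a line of road segments by spawning ActorSpawn actors along the Y axis.
; On BeginPlay it spawns segments until NbrSpawnDisplay reaches NbrSpawnPrepare, advancing the VectorUpdate location by a fixed step after each.
; The AddRoad event appends one more segment at the current VectorUpdate and advances it the same way, leaving the counter untouched.
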(event `self.ReceiveBeginPlay`
  ;[1 1 1] Quand le jeu commence il fait apparaître le nombre de NbrSpawnDisplay
  (while (!= (`self.NbrSpawnDisplay`) (`self.NbrSpawnPrepare`))
    (`|SpawnActorFromClass` (`self.ActorSpawn`) (`KismetMathLibrary.Conv_VectorToTransform` (`self.VectorUpdate`)) "Undefined" "OverrideRootScale" null null)
    (set `self.VectorUpdate` (+ (`self.VectorUpdate`) (0.0 1200.0 0.0)))
    (set `self.NbrSpawnDisplay` (+ (`self.NbrSpawnDisplay`) 1))))

(event `AddRoad`
  ;[1 1 1] Ajout d'une nouvelle route
  (`|SpawnActorFromClass` (`self.ActorSpawn`) (`KismetMathLibrary.Conv_VectorToTransform` (`self.VectorUpdate`)) "Undefined" "OverrideRootScale" null null)
  (set `self.VectorUpdate` (+ (`self.VectorUpdate`) (0.0 1200.0 0.0))))

(fn `UserConstructionScript`)