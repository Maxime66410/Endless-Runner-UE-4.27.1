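; BP_LevelFloor is a floor piece that places a randomly chosen obstacle on itself.
; Its construction script gathers the relative transforms of the right, left and middle spawn components and builds a list of five obstacle classes plus an empty entry.
; It adds one child actor component at a random spawn transform with a random class from that list, so the empty entry can leave the floor clear.
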(fn `SetObstacles`
  (set `self.Obstacles` (`|MakeArray` "/Game/Assets/Obstacle/BP_Obstacle01.BP_Obstacle01_C" "/Game/Assets/Obstacle/BP_Obstacle02.BP_Obstacle02_C" "/Game/Assets/Obstacle/BP_Obstacle03.BP_Obstacle03_C" "/Game/Assets/Obstacle/BP_Obstacle04.BP_Obstacle04_C" "/Game/Assets/Obstacle/BP_Obstacle05.BP_Obstacle05_C" null :!type "Actor Class Reference")))

(fn `SetSpawnPoints`
  (set `self.SpawnPoints` (`|MakeArray` (`SceneComponent.GetRelativeTransform` (`self.SpawnR`)) (`SceneComponent.GetRelativeTransform` (`self.SpawnL`)) (`SceneComponent.GetRelativeTransform` (`self.SpawnM`)))))

(fn `SpawnObstacles`
  (bind _spawnpoints (`self.SpawnPoints`))
  (bind _obstacles (`self.Obstacles`))
  (bind _returnvalue (`AddComponent|NODE_AddChildActorComponent-0` :`RelativeTransform` (`|GetArrayItem` _spawnpoints (`KismetMathLibrary.RandomIntegerInRange` 0 (`KismetArrayLibrary.Array_LastIndex` _spawnpoints)))))
  (`ChildActorComponent.SetChildActorClass` _returnvalue (`|GetArrayItem` _obstacles (`KismetMathLibrary.RandomIntegerInRange` 0 (`KismetArrayLibrary.Array_LastIndex` _obstacles)))))

(fn `UserConstructionScript`
  (`self.SetSpawnPoints`)
  (`self.SetObstacles`)
  (`self.SpawnObstacles`))